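; BP_Coding is a scripting practice Blueprint that exercises basic programming concepts through on-screen printing.
; On BeginPlay it passes two constants to its MyAdd function and prints the returned sum.
; Disconnected EventGraph snippets, partly labelled in Korean, demonstrate variables, branching, a switch on index, array iteration and a loop summing one to ten, but none of them run.
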(event EventBeginPlay
  (bind _result (CallFunction|MyAdd 10 20))
  (Development|PrintString (Utilities|String|ToString(Integer) _result)))

(event Collision|EventActorBeginOverlap
  (params (OtherActor :type Actor%20Object%20Reference)))

(event EventTick
  (params (DeltaSeconds :type Float%20%28single-precision%29)))

(event EventEndPlay
  (params (EndPlayReason :type EEndPlayReason%20Enum :default "Destroyed")))

(fn ConstructionScript)

(fn MyAdd
  (params (A :type Integer) (B :type Integer))
  (return (+ A B)))