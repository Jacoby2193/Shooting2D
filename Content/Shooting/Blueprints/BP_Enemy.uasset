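; BP_Enemy is a shooter enemy that flies in a straight line and destroys both the player and itself on contact.
; At BeginPlay it picks a fixed direction, either toward the player pawn (30% chance) or along its own forward vector.
; Tick moves it along that direction by Speed and delta time without sweep, and an overlap with BP_Player triggers the mutual destruction.
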(event EventBeginPlay
  ;[1 1 1] 태어날 때
  ;  : 방향을 30%확률로 플레이어방향, 나머지는 앞방향으로 정하고
  (if (< (Math|Random|RandomIntegerinRange 0 9) 3)
    (Variables|Default|SetDirection (Math|Vector|Normalize (- (Transformation|GetActorLocation (Game|Player|GetPlayerPawn 0)) (Transformation|GetActorLocation))))
    (else
      (Variables|Default|SetDirection (Transformation|GetActorForwardVector)))))

(event Collision|EventActorBeginOverlap
  (params (OtherActor :type Actor%20Object%20Reference))
  ;[1 1 1] 다른 액터와 부딪힌 순간
  (bind _asbp_player (Utilities|Casting|CastToBP_Player OtherActor))
  (Actor|DestroyActor _asbp_player)
  (Actor|DestroyActor))

(event EventTick
  (params (DeltaSeconds :type Float%20%28single-precision%29))
  ;[1 1 1] 살아가면서 P = P0 + vt
  ;  : 그 방향으로 이동하고싶다.
  (Transformation|SetActorLocation (+ (Transformation|GetActorLocation) (* (Variables|Default|GetDirection) (Variables|Default|GetSpeed) (Utilities|Time|GetWorldDeltaSeconds))) false false))

(event EventEndPlay
  (params (EndPlayReason :type EEndPlayReason%20Enum :default "Destroyed"))
  (switch Utilities|FlowControl|Switch|SwitchonEEndPlayReason EndPlayReason))

(event EventDestroyed)

(fn ConstructionScript)