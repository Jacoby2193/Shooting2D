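; BP_EnemyManager is a spawner actor for the shooting game that keeps creating BP_Enemy instances at its Arrow component's transform.
; BeginPlay starts a timer with a random delay, and each MakeEnemy call spawns an enemy, ignoring collisions, then re-arms the timer with a new random interval.
; An older delta-time accumulator spawn version remains disconnected, and NewFunction is an empty stub.
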(event Custom|MakeEnemy
  (Game|SpawnActorfromClass "/Game/Shooting/Blueprints/BP_Enemy.BP_Enemy_C" (Transformation|GetWorldTransform (Variables|Default|GetArrow)) "AlwaysSpawn" "MultiplyWithRoot" 0 0)
  (Utilities|Time|SetTimerbyEvent (delegate Custom|MakeEnemy) (Math|Random|RandomFloatinRange 1.0 2.0)))

(event EventBeginPlay
  (Utilities|Time|SetTimerbyEvent (delegate Custom|MakeEnemy) (Math|Random|RandomFloatinRange 1.0 2.0)))

(event Collision|EventActorBeginOverlap
  (params (OtherActor :type Actor%20Object%20Reference)))

(event EventTick
  (params (DeltaSeconds :type Float%20%28single-precision%29)))

(fn ConstructionScript)

(fn NewFunction)